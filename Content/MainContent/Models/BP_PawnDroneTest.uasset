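; BP_PawnDroneTest is a test drone pawn whose lift comes from four physics thrusters at the front and rear corners.
; The Throttle input axis sets all four thrusters to the same strength: a constant base plus a small axis-driven offset, scaled by the mass of Cube1.
; It has no steering, stabilisation or per-tick logic, and its construction script is empty.
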(event `InputAxis|Throttle`
  (params (AxisValue :type "Float (single-precision)"))
  (bind _returnvalue (* (+ (* AxisValue 25.0) 970.0) (`PrimitiveComponent.GetMass` (`self.Cube1`))))
  ;[1 1 1] Throttle
  (set `PhysicsThrusterComponent.ThrustStrength` _returnvalue (`self.PhysicsThrusterFR`))
  (set `PhysicsThrusterComponent.ThrustStrength` _returnvalue (`self.PhysicsThrusterFL`))
  (set `PhysicsThrusterComponent.ThrustStrength` _returnvalue (`self.PhysicsThrusterRL`))
  (set `PhysicsThrusterComponent.ThrustStrength` _returnvalue (`self.PhysicsThrusterRR`)))

(fn `UserConstructionScript`)