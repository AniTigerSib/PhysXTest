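; Test drone pawn driven by physics, with throttle-controlled thrust and a mouse-rotated camera arm.
; The Throttle axis sets PhysicsThruster strength as a base value near default gravity plus an input offset, scaled by the Box's mass.
; MouseYaw and MousePitch add relative rotation to the SpringArm, with no pitch clamp.
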(event `InputAxis|Throttle`
  (params (AxisValue :type "Float (single-precision)"))
  ;[1 1 1] Throttle
  (set `PhysicsThrusterComponent.ThrustStrength` (* (+ (* AxisValue 25.0) 970.0) (`PrimitiveComponent.GetMass` (`self.Box`))) (`self.PhysicsThruster`)))

(event `InputAxis|MouseYaw`
  (params (AxisValue :type "Float (single-precision)"))
  ;[1 1 1] MouseCameraControl
  (`SceneComponent.K2_AddRelativeRotation` (`self.SpringArm`) (`KismetMathLibrary.MakeRotator` 0.0 0.0 AxisValue) false false))

(event `InputAxis|MousePitch`
  (params (AxisValue :type "Float (single-precision)"))
  ;[1 1 1] MouseCameraControl
  (`SceneComponent.K2_AddRelativeRotation` (`self.SpringArm`) (`KismetMathLibrary.MakeRotator` 0.0 AxisValue) false false))

(fn `UserConstructionScript`)