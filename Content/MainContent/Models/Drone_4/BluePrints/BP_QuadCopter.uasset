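; Quadcopter drone driven by four physics thrusters, with a mouse-rotated camera arm.
; Each tick, throttle shifts the current and default RPM arrays within a range checked on the first motor, and each RPM scales into thruster strength.
; Pitch or roll input routes RPM through Control, whose mixing logic is unconnected; otherwise all motors reset to the first default.
; Center-of-mass adjustment is also unwired, and Tick prints debug values.
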(event `InputAxis|MouseYaw`
  (params (AxisValue :type "Float (single-precision)"))
  ;[1 1 1] MouseCameraControl
  (`SceneComponent.K2_AddRelativeRotation` (`self.CameraArm`) (`KismetMathLibrary.MakeRotator` 0.0 0.0 AxisValue) false false))

(event `AxisActive`
  (bind _rpm_def (`self.RPM_Def`))
  (bind _rpm (`self.RPM`))
  ;[1 1 1] AxisActivate
  (bind (_rpm_out_fr _rpm_out_fl _rpm_out_rr _rpm_out_rl) (`self.Control` (`|GetArrayItem` _rpm_def) (`|GetArrayItem` _rpm_def 1) (`|GetArrayItem` _rpm_def 2) (`|GetArrayItem` _rpm_def 3) (`self.GetInputAxisValue`) (`self.GetInputAxisValue`)))
  (`KismetArrayLibrary.Array_Set` _rpm 0 _rpm_out_fr)
  (`KismetArrayLibrary.Array_Set` _rpm 1 _rpm_out_fl)
  (`KismetArrayLibrary.Array_Set` _rpm 2 _rpm_out_rr)
  (`KismetArrayLibrary.Array_Set` _rpm 3 _rpm_out_rl))

(event `InputAxis|MousePitch`
  (params (AxisValue :type "Float (single-precision)"))
  ;[1 1 1] MouseCameraControl
  (`SceneComponent.K2_AddRelativeRotation` (`self.CameraArm`) (`KismetMathLibrary.MakeRotator` 0.0 AxisValue) false false))

(event `AxisInactive`
  (bind _rpm (`self.RPM`))
  ;[1 1 1] AxisNonActive
  (for (_ _array_index) _rpm
    (`KismetArrayLibrary.Array_Set` _rpm _array_index (`|GetArrayItem` (`self.RPM_Def`)))))

(event `self.ReceiveBeginPlay`)

(event `self.ReceiveTick`
  (params (DeltaSeconds :type "Float (single-precision)"))
  (bind _returnvalue (`self.GetInputAxisValue`))
  (bind _rpm (`self.RPM`))
  (bind _rpm_def (`self.RPM_Def`))
  (bind _rpm_2 (`self.RPM`))
  ;[1 1 1] DeltaRotationSpeed
  (bind _speed (`self.ThrustAxisToSpeed` (`self.GetInputAxisValue`)))
  (bind _returnvalue_2 (+ _speed (`|GetArrayItem` (`self.RPM`))))
  ;[1 1 1] ThrustSpeed
  (if (and (>= _returnvalue_2 1000.0) (<= _returnvalue_2 2000.0))
    (for (_array_element _array_index) _rpm
      (`KismetArrayLibrary.Array_Set` _rpm _array_index (+ _array_element _speed)))
    (for (_array_element_2 _array_index_2) _rpm_def
      (`KismetArrayLibrary.Array_Set` _rpm_def _array_index_2 (+ _array_element_2 _speed))))
  (`KismetSystemLibrary.PrintString` (`KismetStringLibrary.Conv_DoubleToString` _returnvalue))
  (if (or (!= _returnvalue 0.0) (!= (`self.GetInputAxisValue`) 0.0))
    (`self.AxisActive`)
    (else
      (`self.AxisInactive`)))
  (bind _trust (`self.RPMtoThrust` (`|GetArrayItem` _rpm_2)))
  (bind _output_get (set `PhysicsThrusterComponent.ThrustStrength` _trust (`self.PhysicsThrusterFR`)))
  (`KismetSystemLibrary.PrintString` (`KismetStringLibrary.Conv_DoubleToString` _output_get))
  (bind _trust_2 (`self.RPMtoThrust` (`|GetArrayItem` _rpm_2 1)))
  (set `PhysicsThrusterComponent.ThrustStrength` _trust_2 (`self.PhysicsThrusterFL`))
  (bind _trust_3 (`self.RPMtoThrust` (`|GetArrayItem` _rpm_2 2)))
  (set `PhysicsThrusterComponent.ThrustStrength` _trust_3 (`self.PhysicsThrusterRR`))
  (bind _trust_4 (`self.RPMtoThrust` (`|GetArrayItem` _rpm_2 3)))
  (set `PhysicsThrusterComponent.ThrustStrength` _trust_4 (`self.PhysicsThrusterRL`)))

(fn `ChangeCenterOfMass`
  (params (EngineFR :type "PhysicsThrusterComponent Object Reference") (EngineRR :type "PhysicsThrusterComponent Object Reference"))
  (returns (RelLocY :type "Float (double-precision)") (RelLocZ :type "Float (double-precision)"))
  (bind (_relativelocation_x _relativelocation_y) (`KismetMathLibrary.BreakVector` (`SceneComponent.RelativeLocation` EngineFR)))
  (bind (_relativelocation_x_2 _relativelocation_y_2) (`KismetMathLibrary.BreakVector` (`SceneComponent.RelativeLocation` EngineRR)))
  (return (/ (+ _relativelocation_y _relativelocation_y_2) 2.0) (/ (+ _relativelocation_x _relativelocation_x_2) 2.0)))

(fn `Control`
  (params (RPM_Def_FR :type "Float (double-precision)") (RPM_Def_FL :type "Float (double-precision)") (RPM_Def_RR :type "Float (double-precision)") (RPM_Def_RL :type "Float (double-precision)") (AxisPitch :type "Float (double-precision)") (AxisRoll :type "Float (double-precision)"))
  (returns (RPM_Out_FR :type "Float (double-precision)") (RPM_Out_FL :type "Float (double-precision)") (RPM_Out_RR :type "Float (double-precision)") (RPM_Out_RL :type "Float (double-precision)"))
  (locals (RPM_FR :type "Float (double-precision)") (RPM_FL :type "Float (double-precision)") (RPM_RR :type "Float (double-precision)") (RPM_RL :type "Float (double-precision)") (PitchRatio :type "Float (double-precision)") (RollRatio :type "Float (double-precision)") (PitchDir :type Boolean) (RollDir :type Boolean)))

(fn `RPMtoThrust`
  (params (RotationSpeed :type "Float (double-precision)"))
  (returns (Trust :type "Float (double-precision)"))
  (return (* RotationSpeed (`self.ThrustRatio`))))

(fn `ThrustAxisToSpeed`
  (params (Axis :type "Float (double-precision)"))
  (returns (Speed :type "Float (double-precision)"))
  (return (* Axis 50.0)))

(fn `UserConstructionScript`)