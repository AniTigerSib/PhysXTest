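; Player-controlled quadcopter drone pawn driven by four physics thrusters, with a mouse-rotated camera arm.
; Throttle input accumulates into four rotor RPMs, which Tick scales by ThrustKoef into thruster strengths; front-left reuses rear-left RPM.
; BeginPlay offsets the Box center of mass using the right-side thrusters' averaged location, feeding X into Z.
; Pitch is unfinished: its helper returns zero and positive input enters an empty endless loop.
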(event `InputAxis|MouseYaw`
  (params (AxisValue :type "Float (single-precision)"))
  ;[1 1 1] MouseCameraControl
  (`SceneComponent.K2_AddRelativeRotation` (`self.CameraArm`) (`KismetMathLibrary.MakeRotator` 0.0 0.0 AxisValue) false false))

(event `InputAxis|MousePitch`
  (params (AxisValue :type "Float (single-precision)"))
  ;[1 1 1] MouseCameraControl
  (`SceneComponent.K2_AddRelativeRotation` (`self.CameraArm`) (`KismetMathLibrary.MakeRotator` 0.0 AxisValue) false false))

(event `self.ReceiveBeginPlay`
  ;[1 1 1] Center of Mass
  (bind (_rellocy _rellocz) (`self.ChangeCenterOfMass` (`self.PhysicsThrusterFR`) (`self.PhysicsThrusterRR`)))
  (`PrimitiveComponent.SetCenterOfMass` (`self.Box`) (`KismetMathLibrary.MakeVector` 0.0 _rellocy _rellocz) "None"))

(event `InputAxis|Throttle`
  (params (AxisValue :type "Float (single-precision)"))
  ;[1 1 1] DeltaRotationSpeed
  (bind _speed (`self.ThrustAxisToSpeed` AxisValue))
  ;[1 1 1] ThrustSpeed
  (set `self.RPM_FR` (+ _speed (`self.RPM_FR`)))
  (set `self.RPM_FL` (+ _speed (`self.RPM_FL`)))
  (set `self.RPM_RR` (+ _speed (`self.RPM_RR`)))
  (set `self.RPM_RL` (+ _speed (`self.RPM_RL`))))

(event `InputAxis|Pitch`
  (params (AxisValue :type "Float (single-precision)"))
  (if (not (== AxisValue 0.0))
    (while (> AxisValue 0.0)
      _)))

(event `self.ReceiveTick`
  (params (DeltaSeconds :type "Float (single-precision)"))
  (bind _trust (`self.SpeedToThrust` (`self.RPM_FR`)))
  (set `PhysicsThrusterComponent.ThrustStrength` _trust (`self.PhysicsThrusterFR`))
  (bind _trust_2 (`self.SpeedToThrust` (`self.RPM_RR`)))
  (set `PhysicsThrusterComponent.ThrustStrength` _trust_2 (`self.PhysicsThrusterRR`))
  (bind _trust_3 (`self.SpeedToThrust` (`self.RPM_RL`)))
  (set `PhysicsThrusterComponent.ThrustStrength` _trust_3 (`self.PhysicsThrusterRL`))
  (bind _trust_4 (`self.SpeedToThrust` (`self.RPM_RL`)))
  (set `PhysicsThrusterComponent.ThrustStrength` _trust_4 (`self.PhysicsThrusterFL`)))

(fn `ChangeCenterOfMass`
  (params (EngineFR :type "PhysicsThrusterComponent Object Reference") (EngineRR :type "PhysicsThrusterComponent Object Reference"))
  (returns (RelLocY :type "Float (double-precision)") (RelLocZ :type "Float (double-precision)"))
  (bind (_relativelocation_x _relativelocation_y) (`KismetMathLibrary.BreakVector` (`SceneComponent.RelativeLocation` EngineFR)))
  (bind (_relativelocation_x_2 _relativelocation_y_2) (`KismetMathLibrary.BreakVector` (`SceneComponent.RelativeLocation` EngineRR)))
  (return (/ (+ _relativelocation_y _relativelocation_y_2) 2.0) (/ (+ _relativelocation_x _relativelocation_x_2) 2.0)))

(fn `PitchAxisToSpeed`
  (params (Axis :type "Float (double-precision)"))
  (returns (Speed :type "Float (double-precision)"))
  (return 0.0))

(fn `SpeedToThrust`
  (params (RotationSpeed :type "Float (double-precision)"))
  (returns (Trust :type "Float (double-precision)"))
  (return (* RotationSpeed (`self.ThrustKoef`))))

(fn `ThrustAxisToSpeed`
  (params (Axis :type "Float (double-precision)"))
  (returns (Speed :type "Float (double-precision)"))
  (return (* Axis 50.0)))

(fn `UserConstructionScript`)