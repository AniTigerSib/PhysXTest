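; Player-controlled quadcopter drone pawn that flies on four physics thrusters, with mouse yaw and pitch rotating the camera arm.
; Each tick, throttle shifts all rotor RPMs within a range checked on the front-right rotor, and Control mixes pitch and roll into per-rotor offsets.
; RPMs scale into thruster strengths, resetting to the front-right base when pitch and roll are idle.
; BeginPlay offsets the box's center of mass using the right-side thruster positions.
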(event `AxisActive`
  ;[1 1 1] AxisActivate
  (bind (_rpm_out_fr _rpm_out_fl _rpm_out_rr _rpm_out_rl) (`self.Control` (`self.RPM_Def_FR`) (`self.RPM_Def_FL`) (`self.RPM_Def_RR`) (`self.RPM_Def_RL`) (`self.GetInputAxisValue`) (`self.GetInputAxisValue`)))
  (set `self.RPM_FR` _rpm_out_fr)
  (set `self.RPM_FL` _rpm_out_fl)
  (set `self.RPM_RR` _rpm_out_rr)
  (set `self.RPM_RL` _rpm_out_rl))

(event `InputAxis|MouseYaw`
  (params (AxisValue :type "Float (single-precision)"))
  ;[1 1 1] MouseCameraControl
  (`SceneComponent.K2_AddRelativeRotation` (`self.CameraArm`) (`KismetMathLibrary.MakeRotator` 0.0 0.0 AxisValue) false false))

(event `InputAxis|MousePitch`
  (params (AxisValue :type "Float (single-precision)"))
  ;[1 1 1] MouseCameraControl
  (`SceneComponent.K2_AddRelativeRotation` (`self.CameraArm`) (`KismetMathLibrary.MakeRotator` 0.0 AxisValue) false false))

(event `AxisInactive`
  (bind _rpm_def_fr (`self.RPM_Def_FR`))
  ;[1 1 1] AxisNonActive
  (set `self.RPM_FR` _rpm_def_fr)
  (set `self.RPM_FL` _rpm_def_fr)
  (set `self.RPM_RR` _rpm_def_fr)
  (set `self.RPM_RL` _rpm_def_fr))

(event `self.ReceiveBeginPlay`
  ;[1 1 1] Center of Mass
  (bind (_rellocy _rellocz) (`self.ChangeCenterOfMass` (`self.PhysicsThrusterFR`) (`self.PhysicsThrusterRR`)))
  (`PrimitiveComponent.SetCenterOfMass` (`self.Box`) (`KismetMathLibrary.MakeVector` 0.0 _rellocy _rellocz) "None"))

(event `self.ReceiveTick`
  (params (DeltaSeconds :type "Float (single-precision)"))
  (bind _returnvalue (`self.GetInputAxisValue`))
  ;[1 1 1] DeltaRotationSpeed
  (bind _speed (`self.ThrustAxisToSpeed` (`self.GetInputAxisValue`)))
  (bind _returnvalue_2 (+ _speed (`self.RPM_FR`)))
  ;[1 1 1] ThrustSpeed
  (if (and (>= _returnvalue_2 1000.0) (<= _returnvalue_2 2000.0))
    (set `self.RPM_FR` _returnvalue_2)
    (set `self.RPM_Def_FR` (+ _speed (`self.RPM_Def_FR`)))
    (set `self.RPM_FL` (+ _speed (`self.RPM_FL`)))
    (set `self.RPM_Def_FL` (+ _speed (`self.RPM_Def_FL`)))
    (set `self.RPM_RR` (+ _speed (`self.RPM_RR`)))
    (set `self.RPM_Def_RR` (+ _speed (`self.RPM_Def_RR`)))
    (set `self.RPM_RL` (+ _speed (`self.RPM_RL`)))
    (set `self.RPM_Def_RL` (+ _speed (`self.RPM_Def_RL`))))
  (`KismetSystemLibrary.PrintString` (`KismetStringLibrary.Conv_DoubleToString` _returnvalue))
  (if (or (!= _returnvalue 0.0) (!= (`self.GetInputAxisValue`) 0.0))
    (`self.AxisActive`)
    (else
      (`self.AxisInactive`)))
  (bind _trust (`self.SpeedToThrust` (`self.RPM_FR`)))
  (set `PhysicsThrusterComponent.ThrustStrength` _trust (`self.PhysicsThrusterFR`))
  (bind _trust_2 (`self.SpeedToThrust` (`self.RPM_FL`)))
  (set `PhysicsThrusterComponent.ThrustStrength` _trust_2 (`self.PhysicsThrusterFL`))
  (bind _trust_3 (`self.SpeedToThrust` (`self.RPM_RR`)))
  (set `PhysicsThrusterComponent.ThrustStrength` _trust_3 (`self.PhysicsThrusterRR`))
  (bind _trust_4 (`self.SpeedToThrust` (`self.RPM_RL`)))
  (set `PhysicsThrusterComponent.ThrustStrength` _trust_4 (`self.PhysicsThrusterRL`)))

(fn `ChangeCenterOfMass`
  (params (EngineFR :type "PhysicsThrusterComponent Object Reference") (EngineRR :type "PhysicsThrusterComponent Object Reference"))
  (returns (RelLocY :type "Float (double-precision)") (RelLocZ :type "Float (double-precision)"))
  (bind (_relativelocation_x _relativelocation_y) (`KismetMathLibrary.BreakVector` (`SceneComponent.RelativeLocation` EngineFR)))
  (bind (_relativelocation_x_2 _relativelocation_y_2) (`KismetMathLibrary.BreakVector` (`SceneComponent.RelativeLocation` EngineRR)))
  (return (/ (+ _relativelocation_y _relativelocation_y_2) 2.0) (/ (+ _relativelocation_x _relativelocation_x_2) 2.0)))

(fn `Control`
  (params (RPM_Def_FR :type "Float (double-precision)") (RPM_Def_FL :type "Float (double-precision)") (RPM_Def_RR :type "Float (double-precision)") (RPM_Def_RL :type "Float (double-precision)") (AxisPitch :type "Float (double-precision)") (AxisRoll :type "Float (double-precision)"))
  (returns (RPM_Out_FR :type "Float (double-precision)") (RPM_Out_FL :type "Float (double-precision)") (RPM_Out_RR :type "Float (double-precision)") (RPM_Out_RL :type "Float (double-precision)"))
  (locals (RPM_FR :type "Float (double-precision)") (RPM_FL :type "Float (double-precision)") (RPM_RR :type "Float (double-precision)") (RPM_RL :type "Float (double-precision)") (PitchRatio :type "Float (double-precision)") (RollRatio :type "Float (double-precision)") (PitchDir :type Boolean) (RollDir :type Boolean))
  (bind _rolldir (`local.RollDir`))
  (bind _returnvalue (`KismetMathLibrary.Abs` (`local.PitchRatio`)))
  (bind _returnvalue_2 (`KismetMathLibrary.Abs` (`local.RollRatio`)))
  (bind _returnvalue_3 (`KismetMathLibrary.Abs` (`local.RollRatio`)))
  (bind _returnvalue_4 (`KismetMathLibrary.Abs` (`local.RollRatio`)))
  (bind _returnvalue_5 (`KismetMathLibrary.Abs` (`local.PitchRatio`)))
  (bind _returnvalue_6 (`KismetMathLibrary.Abs` (`local.PitchRatio`)))
  (bind _returnvalue_7 (`KismetMathLibrary.Abs` (`local.PitchRatio`)))
  (bind _returnvalue_8 (`KismetMathLibrary.Abs` (`local.RollRatio`)))
  (bind _returnvalue_9 (`KismetMathLibrary.Abs` (`local.RollRatio`)))
  (bind _returnvalue_10 (`KismetMathLibrary.Abs` (`local.RollRatio`)))
  (bind _returnvalue_11 (+ (`local.RPM_FR`) _returnvalue_7))
  (bind _returnvalue_12 (+ (`local.RPM_FL`) _returnvalue_7))
  (bind _returnvalue_13 (- (`local.RPM_RR`) _returnvalue_7))
  (bind _returnvalue_14 (- (`local.RPM_RL`) _returnvalue_7))
  (bind _returnvalue_15 (- (`local.RPM_FR`) _returnvalue))
  (bind _returnvalue_16 (- (`local.RPM_FL`) _returnvalue))
  (bind _returnvalue_17 (+ (`local.RPM_RR`) _returnvalue))
  (bind _returnvalue_18 (+ (`local.RPM_RL`) _returnvalue))
  (set `local.RPM_FR` RPM_Def_FR)
  (set `local.RPM_FL` RPM_Def_FL)
  (set `local.RPM_RR` RPM_Def_RR)
  (set `local.RPM_RL` RPM_Def_RL)
  (set `local.PitchRatio` (* AxisPitch (`self.PitchRatioRoot`)))
  (set `local.RollRatio` (* AxisRoll (`self.RollRatioRoot`)))
  (set `local.PitchDir` (> AxisPitch 0.0))
  (set `local.RollDir` (> AxisRoll 0.0))
  (if (== AxisPitch 0.0)
    (if (`local.RollDir`)
      (set `local.RPM_FR` (- (`local.RPM_FR`) _returnvalue_3))
      (set `local.RPM_FL` (+ (`local.RPM_FL`) _returnvalue_3))
      (set `local.RPM_RR` (- (`local.RPM_RR`) _returnvalue_3))
      (set `local.RPM_RL` (+ (`local.RPM_RL`) _returnvalue_3))
      (else
        (set `local.RPM_FR` (+ (`local.RPM_FR`) _returnvalue_4))
        (set `local.RPM_FL` (- (`local.RPM_FL`) _returnvalue_4))
        (set `local.RPM_RR` (+ (`local.RPM_RR`) _returnvalue_4))
        (set `local.RPM_RL` (- (`local.RPM_RL`) _returnvalue_4))))
    (elif (== AxisRoll 0.0)
      (if (`local.PitchDir`)
        (set `local.RPM_FR` (+ (`local.RPM_FR`) _returnvalue_5))
        (set `local.RPM_FL` (+ (`local.RPM_FL`) _returnvalue_5))
        (set `local.RPM_RR` (- (`local.RPM_RR`) _returnvalue_5))
        (set `local.RPM_RL` (- (`local.RPM_RL`) _returnvalue_5))
        (else
          (set `local.RPM_FR` (- (`local.RPM_FR`) _returnvalue_6))
          (set `local.RPM_FL` (- (`local.RPM_FL`) _returnvalue_6))
          (set `local.RPM_RR` (+ (`local.RPM_RR`) _returnvalue_6))
          (set `local.RPM_RL` (+ (`local.RPM_RL`) _returnvalue_6))))
      (elif (`local.PitchDir`)
        (if _rolldir
          (set `local.RPM_FR` (- _returnvalue_11 _returnvalue_8))
          (set `local.RPM_FL` (+ _returnvalue_12 _returnvalue_8))
          (set `local.RPM_RR` (- _returnvalue_13 _returnvalue_8))
          (set `local.RPM_RL` (+ _returnvalue_14 _returnvalue_8))
          (else
            (set `local.RPM_FR` (+ _returnvalue_11 _returnvalue_9))
            (set `local.RPM_FL` (- _returnvalue_12 _returnvalue_9))
            (set `local.RPM_RR` (+ _returnvalue_13 _returnvalue_9))
            (set `local.RPM_RL` (- _returnvalue_14 _returnvalue_9))))
        (elif _rolldir
          (set `local.RPM_FR` (- _returnvalue_15 _returnvalue_10))
          (set `local.RPM_FL` (+ _returnvalue_16 _returnvalue_10))
          (set `local.RPM_RR` (- _returnvalue_17 _returnvalue_10))
          (set `local.RPM_RL` (+ _returnvalue_18 _returnvalue_10))
          (else
            (set `local.RPM_FR` (+ _returnvalue_15 _returnvalue_2))
            (set `local.RPM_FL` (- _returnvalue_16 _returnvalue_2))
            (set `local.RPM_RR` (+ _returnvalue_17 _returnvalue_2))
            (set `local.RPM_RL` (- _returnvalue_18 _returnvalue_2)))))))
  (return (`local.RPM_FR`) (`local.RPM_FL`) (`local.RPM_RR`) (`local.RPM_RL`)))

(fn `SpeedToThrust`
  (params (RotationSpeed :type "Float (double-precision)"))
  (returns (Trust :type "Float (double-precision)"))
  (return (* RotationSpeed (`self.ThrustRatio`))))

(fn `ThrustAxisToSpeed`
  (params (Axis :type "Float (double-precision)"))
  (returns (Speed :type "Float (double-precision)"))
  (return (* Axis 50.0)))

(fn `UserConstructionScript`)