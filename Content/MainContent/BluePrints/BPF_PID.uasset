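; Blueprint function asset that provides a generic PID controller calculation.
; PIDCalculations measures error as current minus desired value, integrates it over delta time and differentiates it against the prior error.
; It returns the gain-weighted sum of the three terms.
; The integral and prior error are written back through by-reference parameters, so the caller holds the state between calls, and the integral is not clamped.
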(fn `PIDCalculations`
  (params (CurrentValue :type "Float (double-precision)") (DesiredValue :type "Float (double-precision)") (P :type "Float (double-precision)") (I :type "Float (double-precision)") (D :type "Float (double-precision)") (DeltaTime :type "Float (double-precision)") (IntegralPrior :type "Float (double-precision) (by ref)") (ErrorPrior :type "Float (double-precision) (by ref)"))
  (returns (OutputBias :type "Float (double-precision)"))
  (locals (pIntegral :type "Float (double-precision)") (pErrorPrior :type "Float (double-precision)") (pError :type "Float (double-precision)") (pDerivative :type "Float (double-precision)"))
  (set `local.pErrorPrior` ErrorPrior)
  (set `local.pIntegral` IntegralPrior)
  (bind _output_get (set `local.pError` (- CurrentValue DesiredValue)))
  (set `local.pIntegral` (+ (`local.pIntegral`) (* _output_get DeltaTime)))
  (set `local.pDerivative` (/ (- (`local.pError`) (`local.pErrorPrior`)) DeltaTime))
  (`|VariableSetRef` IntegralPrior (`local.pIntegral`))
  (`|VariableSetRef` ErrorPrior (`local.pError`))
  (return (+ (* P (`local.pError`)) (* I (`local.pIntegral`)) (* D (`local.pDerivative`)))))